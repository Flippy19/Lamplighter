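; BP_Torch is an environment torch whose light color can be picked up by the Lamplighter player's lamp.
; On BeginPlay, its TorchDefaultColor setting (blue, pink or green) sets the point light's color and is cached as the current color.
; LightInteraction copies that color to the player's lamp light and current lamp color, but only when the lamp state is Get.
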(event `/Game/Blueprints/Interfaces/I_Light.Light Interaction`
  (bind _current_light_color (`self.Current Light Color`))
  ;[0.2076 0.07424 0.4072] Set Lamp Light Color
  (bind _aschar_lamplighter (cast `/Game/Blueprints/Player/Char_Lamplighter` (`GameplayStatics.GetPlayerCharacter` 0)))
  (switch `/Game/Blueprints/Player/LampStates` (`/Game/Blueprints/Player/Char_Lamplighter.Lamp States` _aschar_lamplighter)
    (:`NewEnumerator1`
      (`LightComponent.SetLightColor` (`/Game/Blueprints/Player/Char_Lamplighter.Lamp PointLight` _aschar_lamplighter) _current_light_color true)
      (set `/Game/Blueprints/Player/Char_Lamplighter.Current Lamp Color` _current_light_color _aschar_lamplighter))))

(event `self.ReceiveBeginPlay`
  (bind _torch_green_color (`self.Torch Green Color`))
  (bind _torch_blue_color (`self.Torch Blue Color`))
  (bind _pointlight (`self.PointLight`))
  (bind _torch_pink_color (`self.Torch Pink Color`))
  ;[0.1597 0.1511 1] Set Torch Light Color
  (switch `/Game/Blueprints/Environment/TorchColors` (`self.Torch Default Color`)
    (:`NewEnumerator0`
      (`LightComponent.SetLightColor` _pointlight _torch_blue_color true)
      (set `self.Current Light Color` _torch_blue_color))
    (:`NewEnumerator1`
      (`LightComponent.SetLightColor` _pointlight _torch_pink_color true)
      (set `self.Current Light Color` _torch_pink_color))
    (:`NewEnumerator2`
      (`LightComponent.SetLightColor` _pointlight _torch_green_color true)
      (set `self.Current Light Color` _torch_green_color))))

(fn `UserConstructionScript`)