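; BP_Chest_Buttons is a chest whose lock depends on a set of BP_Button actors.
; On BeginPlay it registers itself as ChestRef on each button in its Buttons array.
; Its Check event loops through them, calling Unlock and Open at each active button and locking at the first inactive one.
; Open can therefore fire before every button has been checked.
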(event `self.ReceiveBeginPlay`
  (for _array_element (`self.Buttons`)
    (bind _asbp_button (cast `/Game/Blueprints/Environment/Doors/Buttons/BP_Button` _array_element))
    (set `/Game/Blueprints/Environment/Doors/Buttons/BP_Button.Chest Ref` self _asbp_button)))

(event `Check`
  (bind _buttons (`self.Buttons`))
  (for _index (range (+ (`KismetArrayLibrary.Array_Length` _buttons) 1))
    (bind _asbp_button (cast `/Game/Blueprints/Environment/Doors/Buttons/BP_Button` (`|GetArrayItem` _buttons _index)))
    (if (`/Game/Blueprints/Environment/Doors/Buttons/BP_Button.IsActive` _asbp_button)
      (`self.Unlock`)
      (`self.Open`)
      (else
        (`self.Lock`)
        (break)))))

(event `Unlock`
  (set `self.Locked` false))

(event `Lock`
  (set `self.Locked` true))

(fn `UserConstructionScript`
  (`parent.UserConstructionScript`))