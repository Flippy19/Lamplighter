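; BP_Button is a toggle button in the environment that works with a referenced door.
; On Interaction, if the door reference is valid, it flips IsActive and swaps the cube's material between active and inactive looks.
; It then calls Check on the door after each toggle, leaving the door to evaluate the new state.
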(event `/Game/Blueprints/Interfaces/I_Interactable.Interaction`
  (`/Engine/EditorBlueprintResources/StandardMacros.IsValid` (`self.Door Ref`)
    (:`Is Valid`
      (if (`self.IsActive`)
        (set `self.IsActive` false)
        (set `self.Material` "/Game/Materials/M_Button_NotActive.M_Button_NotActive")
        (else
          (set `self.IsActive` true)
          (set `self.Material` "/Game/Materials/M_Button_Active.M_Button_Active")))
      (`PrimitiveComponent.SetMaterial` (`self.Cube`) 0 (`self.Material`))
      (`/Game/Blueprints/Environment/BP_Door.Check` (`self.Door Ref`)))))

(fn `UserConstructionScript`)