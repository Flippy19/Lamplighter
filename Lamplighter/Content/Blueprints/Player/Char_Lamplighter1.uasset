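; Player character for the lamplighter, handling movement, timeline-driven sprint with FOV change, lantern control and interaction.
; Set/Get inputs play a timeline that moves and brightens the lamp, then messages the I_Light actor tracked by an overlap radius; Reset restores the default color.
; A camera line trace messages I_Interactable actors.
; Journal and map widgets toggle mutually exclusively, and the JournalBlock macro gates most gameplay input while either is open.
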(event `self.Lamp Interaction Radius.OnComponentBeginOverlap`
  (params (OverlappedComponent :type "PrimitiveComponent Object Reference") (OtherActor :type "Actor Object Reference") (OtherComp :type "PrimitiveComponent Object Reference") (OtherBodyIndex :type Integer) (bFromSweep :type Boolean) (SweepResult :type "HitResult Structure (by ref)"))
  ;[0.3712 0.04922 0.03445] Checking if lantern or torch is in the Light Interaction Radius
  (if (`KismetSystemLibrary.DoesImplementInterface` OtherActor "/Game/Blueprints/Interfaces/I_Light.I_Light_C")
    (set `self.Lamp Interaction Object Ref` OtherActor)
    (switch `/Game/Blueprints/Player/LampStates` (`self.Lamp States`)
      (:`NewEnumerator0`
        (`self.Lamp Set Light`))
      (:`NewEnumerator1`
        (`self.Lamp Get Light`)))))

(event `self.Lamp Interaction Radius.OnComponentEndOverlap`
  (params (OverlappedComponent :type "PrimitiveComponent Object Reference") (OtherActor :type "Actor Object Reference") (OtherComp :type "PrimitiveComponent Object Reference") (OtherBodyIndex :type Integer))
  ;[0.3712 0.04922 0.03445] Checking if lantern or torch is in the Light Interaction Radius
  (if (== (`self.Lamp Interaction Object Ref`) OtherActor)
    (set `self.Lamp Interaction Object Ref` null)))

(event `InputAction|Set Light`
  (params (Key :type "Key Structure"))
  ;[0.9115 0.07121 0.1861] Lamp Logic
  (:`Pressed`
    (`self.JournalBlock`
      (:`false`
        (if (`self.Can Change State`)
          (set `self.Lamp States` "NewEnumerator0")
          (bind (_direction _lamp_point_movement _light_intensity_change) (`Timeline|Lamp Timeline` :!label _label)
            (:`Update`
              (`self.Lamp Change Light Intensity` _light_intensity_change)
              (`self.SetTransform` _lamp_point_movement))
            (:`Finished`
              (`self.Lamp Switch States` (`self.Lamp States`))))))))
  (:`Released`
    (set `self.Lamp States` "NewEnumerator2" :!label _label_2)
    (goto _label :!via `Reverse`)))

(event `InputAction|Get Light`
  (params (Key :type "Key Structure"))
  ;[0.9115 0.07121 0.1861] Lamp Logic
  (:`Pressed`
    (`self.JournalBlock`
      (:`false`
        (if (`self.Can Change State`)
          (set `self.Lamp States` "NewEnumerator1")
          (goto _label)))))
  (:`Released`
    (goto _label_2)))

(event `InputAction|Map`
  (params (Key :type "Key Structure"))
  (bind _mapwidget (`self.MapWidget`))
  ;[1 0.1316 0.08185] Map Widget
  (:`Pressed`
    (if (not (`self.IsJournalActive`))
      (`/Engine/EditorBlueprintResources/StandardMacros.FlipFlop`
        (:`A`
          (`Widget.SetVisibility` _mapwidget "Visible")
          (set `self.IsMapActive` true))
        (:`B`
          (`Widget.SetVisibility` _mapwidget "Hidden")
          (set `self.IsMapActive` false))))))

(event `InputAction|Reset Light`
  (params (Key :type "Key Structure"))
  ;[0.9115 0.07121 0.1861] Lamp Logic
  ;;[1 1 1] Reset Lamp Color
  (:`Pressed`
    (`self.Lamp Reset Light`)))

(event `InputAction|Sprint`
  (params (Key :type "Key Structure"))
  ;[1 0.149 0.8392] Szprint
  (:`Pressed`
    (`self.JournalBlock`
      (:`false`
        (if (!= (`MovementComponent.Velocity` (`self.CharacterMovement`)) (0.0 0.0 0.0))
          (bind (_direction _runspeed _fov) (`Timeline|Timeline` :!label _label_3)
            (:`Update`
              (set `CharacterMovementComponent.MaxWalkSpeed` _runspeed (`self.CharacterMovement`))
              (`CameraComponent.SetFieldOfView` (`self.Camera`) _fov)))))))
  (:`Released`
    (goto _label_3 :!via `Reverse`)))

(event `self.ReceiveBeginPlay`
  ;[1 0.4612 0.145] Add Widget to Viewport
  (bind _returnvalue (`|CreateWidget` "/Game/UI/Blueprints/BP_Journal.BP_Journal_C"))
  (bind _output_get (set `self.JournalWidget` _returnvalue))
  (`UserWidget.AddToViewport` _output_get 0)
  (`Widget.SetVisibility` _output_get "Hidden")
  (bind _returnvalue_2 (`|CreateWidget` "/Game/UI/Blueprints/BP_Map.BP_Map_C"))
  (bind _output_get_2 (set `self.MapWidget` _returnvalue_2))
  (`UserWidget.AddToViewport` _output_get_2 0)
  (`Widget.SetVisibility` _output_get_2 "Hidden"))

(event `InputAxis|MoveForward`
  (params (AxisValue :type "Float (single-precision)"))
  ;[0.3772 0.1153 1] Movement
  (`self.JournalBlock`
    (:`false`
      (`self.AddMovementInput` (`SceneComponent.GetForwardVector` (`self.CapsuleComponent`)) (* AxisValue (`GameplayStatics.GetWorldDeltaSeconds`) (`self.Movement Multiplier`))))))

(event `InputAxis|LookUp`
  (params (AxisValue :type "Float (single-precision)"))
  ;[0.03372 0.226 1] Camera
  (`self.JournalBlock`
    (:`false`
      (`self.AddControllerPitchInput` (* AxisValue (`self.Mouse Sensitivity`))))))

(event `InputAxis|MoveRight`
  (params (AxisValue :type "Float (single-precision)"))
  ;[0.3772 0.1153 1] Movement
  (`self.JournalBlock`
    (:`false`
      (`self.AddMovementInput` (`SceneComponent.GetRightVector` (`self.CapsuleComponent`)) (* AxisValue (`GameplayStatics.GetWorldDeltaSeconds`) (`self.Movement Multiplier`))))))

(event `InputAxis|Turn`
  (params (AxisValue :type "Float (single-precision)"))
  ;[0.03372 0.226 1] Camera
  (`self.JournalBlock`
    (:`false`
      (`self.AddControllerYawInput` (* AxisValue (`self.Mouse Sensitivity`))))))

(event `InputAction|Journal`
  (params (Key :type "Key Structure"))
  (bind _returnvalue (`GameplayStatics.GetPlayerController` 0))
  (bind _journalwidget (`self.JournalWidget`))
  ;[1 0.7352 0.1944] Journal Widget
  (:`Pressed`
    (if (not (`self.IsMapActive`))
      (`/Engine/EditorBlueprintResources/StandardMacros.FlipFlop`
        (:`A`
          (`Widget.SetVisibility` _journalwidget "Visible")
          (set `self.IsJournalActive` true)
          (set `PlayerController.bShowMouseCursor` true _returnvalue))
        (:`B`
          (`Widget.SetVisibility` _journalwidget "Hidden")
          (set `self.IsJournalActive` false)
          (set `PlayerController.bShowMouseCursor` false _returnvalue))))))

(event `InputAction|Interaction`
  (params (Key :type "Key Structure"))
  (bind _camera (`self.Camera`))
  (bind _returnvalue (`SceneComponent.K2_GetComponentLocation` _camera))
  ;[0.1656 0.9602 1] Interaction LineTrace By Channel
  (:`Pressed`
    (`self.JournalBlock`
      (:`false`
        (bind _outhit (`KismetSystemLibrary.LineTraceSingle` :`Start` _returnvalue :`End` (+ _returnvalue (* (`KismetMathLibrary.GetForwardVector` (`SceneComponent.K2_GetComponentRotation` _camera)) (`self.Raycast Lenght`))) :`TraceChannel` "TraceTypeQuery1" :`DrawDebugType` "ForDuration"))
        (set `self.Hit Actor Ref` (`.HitActor` (`GameplayStatics.BreakHitResult` _outhit)))
        (`self.Send Interaction Message`)))))

(event `Send Interaction Message`
  (bind _hit_actor_ref (`self.Hit Actor Ref`))
  ;[0.1199 0.7552 0.09833] Send Interaction Message
  (`self.JournalBlock`
    (:`false`
      (if (`KismetSystemLibrary.DoesImplementInterface` _hit_actor_ref "/Game/Blueprints/Interfaces/I_Interactable.I_Interactable_C")
        (message `/Game/Blueprints/Interfaces/I_Interactable.Interaction` _hit_actor_ref)
        (`KismetSystemLibrary.PrintString` (`KismetStringLibrary.Concat_StrStr` "Interaction with: " (`KismetSystemLibrary.GetDisplayName` _hit_actor_ref)))))))

(fn `Lamp Change Light Intensity`
  (params (LightIntensity :type "Float (double-precision)"))
  (`LightComponent.SetIntensity` (`self.Lamp PointLight`) LightIntensity))

(fn `Lamp Get Light`
  (bind _lamp_interaction_object_ref (`self.Lamp Interaction Object Ref`))
  (`/Engine/EditorBlueprintResources/StandardMacros.IsValid` _lamp_interaction_object_ref
    (:`Is Valid`
      (message `/Game/Blueprints/Interfaces/I_Light.Light Interaction` _lamp_interaction_object_ref))))

(fn `Lamp Reset Light`
  (bind _output_get (set `self.Current Lamp Color` (`self.Defalut Lamp Color`)))
  (`LightComponent.SetLightColor` (`self.Lamp PointLight`) _output_get true))

(fn `Lamp Set Light`
  (bind _lamp_interaction_object_ref (`self.Lamp Interaction Object Ref`))
  (`/Engine/EditorBlueprintResources/StandardMacros.IsValid` _lamp_interaction_object_ref
    (:`Is Valid`
      (message `/Game/Blueprints/Interfaces/I_Light.Light Interaction` _lamp_interaction_object_ref))))

(fn `Lamp Switch States`
  (params (`Lamp States` :type "/Game/Blueprints/Player/LampStates Enum" :default "NewEnumerator0"))
  (switch `/Game/Blueprints/Player/LampStates` `Lamp States`
    (:`NewEnumerator0`
      (set `self.Can Change State` false)
      (`self.Lamp Set Light`))
    (:`NewEnumerator1`
      (set `self.Can Change State` false)
      (`self.Lamp Get Light`))
    (:`NewEnumerator2`
      (set `self.Can Change State` true))))

(fn `UserConstructionScript`)