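; BP_Door is an interactable rotating door that stays unlocked only while all its linked buttons are active.
; BeginPlay gives each BP_Button a reference to the door.
; Check scans the buttons, unlocking if all are active, otherwise locking and closing.
; Interaction toggles an unlocked door through a timeline driving its yaw; Close only reverses it while AllButtonsActive is set, which Check clears after closing.
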(event `self.ReceiveBeginPlay`
  ;[1 1 1] Set Door Ref in every connected button to: this object
  (for _array_element (`self.Buttons`)
    (bind _asbp_button (cast `/Game/Blueprints/Environment/Doors/Buttons/BP_Button` _array_element))
    (set `/Game/Blueprints/Environment/Doors/Buttons/BP_Button.Door Ref` self _asbp_button)))

(event `/Game/Blueprints/Interfaces/I_Interactable.Interaction`
  ;[1 1 1] Check if doors are locked and opened
  (if (`self.Locked`)
    _
    (elif (`self.IsOpen`)
      (`self.Close`)
      (else
        (`self.Open`)))))

(event `Check`
  (bind _buttons (`self.Buttons`))
  ;[1 1 1] If every Button is active > Unlock the door
  (for _index (range (+ (`KismetArrayLibrary.Array_Length` _buttons) 1))
    (bind _asbp_button (cast `/Game/Blueprints/Environment/Doors/Buttons/BP_Button` (`|GetArrayItem` _buttons _index)))
    (if (`/Game/Blueprints/Environment/Doors/Buttons/BP_Button.IsActive` _asbp_button)
      (`self.Unlock`)
      (set `self.AllButtonsActive` true)
      (else
        (`self.Lock`)
        (`self.Close`)
        (set `self.AllButtonsActive` false)
        (break)))))

(event `Unlock`
  ;[1 1 1] Open and Close
  (set `self.Locked` false))

(event `Lock`
  ;[1 1 1] Open and Close
  (set `self.Locked` true))

(event `Open`
  ;[1 1 1] Open and Close
  (set `self.IsOpen` true)
  (bind (_direction _rotate_door) (`Timeline|Open/Close` :!label _label)
    (:`Update`
      (`SceneComponent.K2_SetRelativeRotation` (`self.Door`) (`KismetMathLibrary.MakeRotator` 0.0 0.0 (* _rotate_door 90.0)) false false))))

(event `Close`
  ;[1 1 1] Open and Close
  (if (`self.AllButtonsActive`)
    (set `self.IsOpen` false)
    (goto _label :!via `Reverse`)))

(fn `UserConstructionScript`)