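; BP_Door is a lockable door gated by a set of BP_Button actors.
; On BeginPlay it registers itself as each button's DoorRef.
; Check unlocks it while scanning active buttons, but locks and closes it at the first inactive one.
; Interaction toggles an unlocked door open or closed by switching collision and swapping materials, while a separate indicator's material shows lock state.
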(event `self.ReceiveBeginPlay`
  ;[1 1 1] Set Door Ref in every connected button to: this object
  (for _array_element (`self.Buttons`)
    (bind _asbp_button (cast `/Game/Blueprints/Environment/BP_Button` _array_element))
    (set `/Game/Blueprints/Environment/BP_Button.Door Ref` self _asbp_button)))

(event `/Game/Blueprints/Interfaces/I_Interactable.Interaction`
  ;[1 1 1] Check if doors are locked and opened
  (if (`self.Locked`)
    _
    (elif (`self.IsOpen`)
      (`self.Close`)
      (else
        (`self.Open`)))))

(event `Check`
  (bind _buttons (`self.Buttons`))
  ;[1 1 1] If every Button is active > Unlock the door
  (for _index (range (+ (`KismetArrayLibrary.Array_Length` _buttons) 1))
    (bind _asbp_button (cast `/Game/Blueprints/Environment/BP_Button` (`|GetArrayItem` _buttons _index)))
    (if (`/Game/Blueprints/Environment/BP_Button.IsActive` _asbp_button)
      (`self.Unlock`)
      (else
        (`self.Lock`)
        (`self.Close`)
        (break)))))

(event `Unlock`
  ;[1 1 1] Lock and Unlock
  (set `self.Locked` false)
  (set `self.LockMaterial` "/Game/Materials/M_Button_Active.M_Button_Active")
  (`PrimitiveComponent.SetMaterial` (`self.LockIndicator`) 0 (`self.LockMaterial`) :!label _label))

(event `Lock`
  ;[1 1 1] Lock and Unlock
  (set `self.Locked` true)
  (set `self.LockMaterial` "/Game/Materials/M_Button_NotActive.M_Button_NotActive")
  (goto _label))

(event `Open`
  ;[1 1 1] Open and Close
  (set `self.IsOpen` true)
  (set `self.Door Material` "/Game/Materials/M_Door_Opened.M_Door_Opened")
  (`PrimitiveComponent.SetCollisionEnabled` (`self.Door`) "NoCollision")
  (`PrimitiveComponent.SetCollisionEnabled` (`self.LockIndicator`) "NoCollision")
  (`PrimitiveComponent.SetMaterial` (`self.Door`) 0 (`self.Door Material`) :!label _label_2))

(event `Close`
  ;[1 1 1] Open and Close
  (set `self.IsOpen` false)
  (set `self.Door Material` "/Game/Materials/M_Door_Closed.M_Door_Closed")
  (`PrimitiveComponent.SetCollisionEnabled` (`self.Door`) "QueryAndPhysics")
  (`PrimitiveComponent.SetCollisionEnabled` (`self.LockIndicator`) "QueryAndPhysics")
  (goto _label_2))

(fn `UserConstructionScript`)