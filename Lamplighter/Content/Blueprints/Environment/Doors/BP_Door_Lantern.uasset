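; Door Blueprint linked to two lanterns, toggling open or closed on interaction unless locked.
; On BeginPlay it registers itself as DoorRef on both BP_Lantern actors, then derives door colors from their Blue, Pink or Green settings.
; Every Lantern2Color case copies DoorColor1 into DoorColor2, so both colors follow the first lantern.
; CheckLanterns is an empty stub, and nothing here changes the lock state.
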(event `self.ReceiveBeginPlay`
  (`self.LantersRef`)
  (`self.LantersColor`))

(event `/Game/Blueprints/Interfaces/I_Interactable.Interaction`
  (if (`self.Locked`)
    _
    (elif (`self.IsOpen`)
      (`self.Close`)
      (else
        (`self.Open`)))))

(event `LantersColor`
  (switch `/Game/Blueprints/Environment/TorchColors` (`self.Lantern 1 Color`)
    (:`NewEnumerator0`
      (bind _output_get (set `self.Door Color 1` (struct :`G` 0.135633 :`B` 1.0 :`A` 1.0))))
    (:`NewEnumerator1`
      (bind _output_get_2 (set `self.Door Color 1` (struct :`R` 1.0 :`B` 0.737911 :`A` 1.0))))
    (:`NewEnumerator2`
      (bind _output_get_3 (set `self.Door Color 1` (struct :`G` 0.938686 :`B` 1.0 :`A` 1.0)))))
  (switch `/Game/Blueprints/Environment/TorchColors` (`self.Lantern 2 Color`)
    (:`NewEnumerator0`
      (set `self.Door Color 2` _output_get))
    (:`NewEnumerator1`
      (set `self.Door Color 2` _output_get_2))
    (:`NewEnumerator2`
      (set `self.Door Color 2` _output_get_3))))

(event `LantersRef`
  (bind _asbp_lantern (cast `/Game/Blueprints/Environment/BP_Lantern` (`self.Lantern 1`)))
  (set `/Game/Blueprints/Environment/BP_Lantern.DoorRef` self _asbp_lantern)
  (bind _asbp_lantern_2 (cast `/Game/Blueprints/Environment/BP_Lantern` (`self.Lantern 2`)))
  (set `/Game/Blueprints/Environment/BP_Lantern.DoorRef` self _asbp_lantern_2))

(event `CheckLanterns`)

(fn `UserConstructionScript`
  (`parent.UserConstructionScript`))