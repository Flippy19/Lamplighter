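; A door variant that opens through light interaction when the player's lamp color matches the door's unlock color.
; On BeginPlay, the unlock color enum (blue, pink or green) sets the required torch color and the matching material on the color indicator.
; LightInteraction checks the Lamplighter player's lamp state and current color, then calls Open if both match.
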(event `self.ReceiveBeginPlay`
  (switch `/Game/Blueprints/Environment/TorchColors` (`self.UnlockColorEnum`)
    (:`NewEnumerator0`
      (set `self.UnlockColor` (`self.Torch Blue Color`))
      (set `self.MaterialIndex` 0))
    (:`NewEnumerator1`
      (set `self.UnlockColor` (`self.Torch Pink Color`))
      (set `self.MaterialIndex` 1))
    (:`NewEnumerator2`
      (set `self.UnlockColor` (`self.Torch Green Color`))
      (set `self.MaterialIndex` 2)))
  (`PrimitiveComponent.SetMaterial` (`self.Color Indicator`) 0 (`|GetArrayItem` (`self.UnlockMaterials`) (`self.MaterialIndex`))))

(event `/Game/Blueprints/Interfaces/I_Light.Light Interaction`
  (bind _aschar_lamplighter (cast `/Game/Blueprints/Player/Char_Lamplighter` (`GameplayStatics.GetPlayerCharacter` 0)))
  (if (`|EnumEquality` (`/Game/Blueprints/Player/Char_Lamplighter.Lamp States` _aschar_lamplighter) "NewEnumerator0")
    (if (== (`/Game/Blueprints/Player/Char_Lamplighter.Current Lamp Color` _aschar_lamplighter) (`self.UnlockColor`))
      (`self.Open`))))

(fn `UserConstructionScript`
  (`parent.UserConstructionScript`))