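; BP_Button_Church is an interactable environment button that switches between active and inactive states.
; On Interaction, if either a door or a chest reference is valid, it toggles IsActive, swaps the button material and rotates the button to match.
; The logic that would call Check on the linked door or chest is disconnected, so this graph never notifies them.
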(event `/Game/Blueprints/Interfaces/I_Interactable.Interaction`
  (`/Engine/EditorBlueprintResources/StandardMacros.IsValid` (`self.Door Ref`)
    (:`Is Valid`
      _)
    (:`Is Not Valid`
      (`/Engine/EditorBlueprintResources/StandardMacros.IsValid` (`self.Chest Ref`)
        (:`Is Valid`
          _))))
  (if (`self.IsActive`)
    (set `self.IsActive` false)
    (`PrimitiveComponent.SetMaterial` (`self.Button`) 0 "/Game/Materials/M_Button_NotActive.M_Button_NotActive")
    (`SceneComponent.K2_SetRelativeRotation` (`self.Button`) (struct :`Pitch` 335.0 :`Yaw` 540.0 :`Roll` 180.0) false false)
    (else
      (set `self.IsActive` true)
      (`PrimitiveComponent.SetMaterial` (`self.Button`) 0 "/Game/Materials/M_Button_Active.M_Button_Active")
      (`SceneComponent.K2_SetRelativeRotation` (`self.Button`) (struct :`Pitch` 380.0 :`Yaw` 540.0 :`Roll` 180.0) false false))))

(fn `UserConstructionScript`
  (`parent.UserConstructionScript`))