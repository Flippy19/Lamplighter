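; BP_Chest_Lamp is a chest that opens when the Lamplighter player's lamp matches its unlock color.
; BeginPlay maps the blue, pink or green enum to an unlock color and a material index.
; LightInteraction checks the player's lamp state and current lamp color against that color before calling Open.
; Open plays a timeline that rotates the lid on roll, then marks the chest open when finished.
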(event `self.ReceiveBeginPlay`
  (switch `/Game/Blueprints/Environment/TorchColors` (`self.UnlockColorEnum`)
    (:`NewEnumerator0`
      (set `self.UnlockColor` (`self.Torch Blue Color`))
      (set `self.MaterialIndex` 0))
    (:`NewEnumerator1`
      (set `self.UnlockColor` (`self.Torch Pink Color`))
      (set `self.MaterialIndex` 1))
    (:`NewEnumerator2`
      (set `self.UnlockColor` (`self.Torch Green Color`))
      (set `self.MaterialIndex` 2))))

(event `/Game/Blueprints/Interfaces/I_Light.Light Interaction`
  (bind _aschar_lamplighter (cast `/Game/Blueprints/Player/Char_Lamplighter` (`GameplayStatics.GetPlayerCharacter` 0)))
  (if (`|EnumEquality` (`/Game/Blueprints/Player/Char_Lamplighter.Lamp States` _aschar_lamplighter) "NewEnumerator0")
    (if (== (`/Game/Blueprints/Player/Char_Lamplighter.Current Lamp Color` _aschar_lamplighter) (`self.UnlockColor`))
      (`self.Open`))))

(event `Open`
  (if (not (`self.isOpen`))
    (bind (_direction _rotate_lid) (`Timeline|Opening`)
      (:`Update`
        (`SceneComponent.K2_SetRelativeRotation` (`self.Lid`) (`KismetMathLibrary.MakeRotator` (* _rotate_lid -90.0)) false false))
      (:`Finished`
        (set `self.isOpen` true)))))

(fn `UserConstructionScript`)